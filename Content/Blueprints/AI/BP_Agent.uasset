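; BP_Agent is an AI agent Blueprint set up for custom navigation, though its pathfinding is unfinished.
; On BeginPlay it caches the first CustomNavigationData actor as its Navmesh.
; Disconnected EventGraph nodes would pass that, its location and a Target to BuildPath, which is empty, and draw the result as debug lines.
; Tick and the construction script do nothing, with unwired TextRenderActor cleanup left in the latter.
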(event `self.ReceiveBeginPlay`
  (bind _outactors (`GameplayStatics.GetAllActorsOfClass` "/Script/Navmesh_Generation.CustomNavigationData"))
  (set `self.Navmesh` (`|GetArrayItem` _outactors)))

(event `self.ReceiveTick`
  (params (DeltaSeconds :type "Float (single-precision)")))

(fn `BuildPath`)

(fn `UserConstructionScript`)